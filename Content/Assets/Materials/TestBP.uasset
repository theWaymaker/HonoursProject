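; Planetarium actor that runs Moon and Jupiter narration and rotation stages, then an ending sequence.
; When each audio finishes, it shows a spacebar icon and spins the Rotunda by timeline until a stop event eases it to a set rotation.
; The Moon stop triggers the character's Jupiter mini-game.
; The Jupiter stop posts the timer to a Discord webhook, plays peat audio, switches cameras, raises and lowers LandscapeLift, and binds camera reset.
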(event Custom|StartMoving
  (bind _returnvalue (UserInterface|CreateWidget "/Game/Widgets/SpacebarIcon.SpacebarIcon_C"))
  (Variables|Default|SetSpaceWidgetRef _returnvalue)
  (UserInterface|Viewport|AddtoViewport _returnvalue 0)
  (bind _rotationrate (Timeline|Timeline Play)
    (:Update
      (Transformation|SetRelativeRotation (Variables|Default|GetRotunda) (Math|Rotator|Lerp(Rotator) (Variables|Default|GetStartRotation) (Variables|Default|GetEndRotation) _rotationrate) false false))))

(event Custom|StopMoving2
  (bind _timerref (Variables|Default|GetTimerRef))
  (bind _timeminutes (Variables|/Game/FirstPerson/Blueprints/Timer.Timer_C|GetTimeMinutes _timerref))
  (bind _timeseconds (Variables|/Game/FirstPerson/Blueprints/Timer.Timer_C|GetTimeSeconds _timerref))
  (bind _returnvalue (Utilities|String|ToString(Integer) _timeminutes))
  (bind _returnvalue_2 (Utilities|String|ToString(Integer) _timeseconds))
  (Variables|Default|SetCurrentRotation (Variables|/Script/Engine.SceneComponent|GetRelativeRotation (Variables|Default|GetRotunda)))
  (Utilities|FlowControl|Sequence
    (:then_0
      (bind _rotationrate (Timeline|Timeline_0 Stop)
        (:Update
          (Transformation|SetRelativeRotation (Variables|Default|GetRotunda) (Math|Rotator|Lerp(Rotator) (Variables|Default|GetMoonRotation) (Math|Rotator|MakeRotator 0.0 0.0 (+ (.yaw (Variables|Default|GetMoonRotation)) 3.6e+02)) _rotationrate) false false))))
    (:then_1
      (bind _slowrate (Timeline|Timeline_1 Play)
        (:Update
          (Transformation|SetRelativeRotation (Variables|Default|GetRotunda) (Math|Rotator|Lerp(Rotator) (Variables|Default|GetCurrentRotation) "0.000000,50.000000,0.000000" _slowrate) false false)
          (Widget|RemovefromParent (Variables|Default|GetSpaceWidgetRef)))
        (:Finished
          (Utilities|FlowControl|Delay 1.0)
          (Rendering|SetVisibility (Variables|/Game/FirstPerson/Blueprints/TextRenderJupiterBP.TextRenderJupiterBP_C|GetText3D (Variables|Default|GetJupiterTextRef)) false false)
          (if (< _timeseconds 10)
            (Class|DiscordMessengerBPLibrary|SendDiscordMessage "https://discord.com/api/webhooks/1089919669479153808/YOL72xxdeQtgSDdMLGKN487o-ZjgjsYcFaU3AafmQ2GCWnPC3DYFIiv8SImxikTTgqKV" (Utilities|String|Append (Utilities|String|Append _returnvalue ":" (Utilities|String|Append "0" _returnvalue_2)) "Activity Completed"))
            (else
              (Class|DiscordMessengerBPLibrary|SendDiscordMessage "https://discord.com/api/webhooks/1089919669479153808/YOL72xxdeQtgSDdMLGKN487o-ZjgjsYcFaU3AafmQ2GCWnPC3DYFIiv8SImxikTTgqKV" (Utilities|String|Append (Utilities|String|Append _returnvalue ":" _returnvalue_2) "Activity Completed"))))
          (Audio|Components|Audio|Play (Variables|Default|GetCoveredInPeat) 0.0)
          (Game|Player|SetViewTargetwithBlend (Game|GetPlayerController 0) (Variables|Default|GetCameraPeatRef) 2.0 "VTBlend_Linear" 0.0 false)
          (Utilities|FlowControl|Delay 12.0)
          (Default|RaiseHell (Variables|Default|GetLandscapeLiftRef))
          (Utilities|FlowControl|Delay 8.0)
          (Default|LowerHell (Variables|Default|GetLandscapeLiftRef))
          (EventDispatchers|BindEventtoOnAudioFinished (Variables|Default|GetCoveredInPeat) (delegate Custom|ResetCamera)))))))

(event Custom|PlayMoonAudio
  (Audio|Components|Audio|Play (Variables|Default|GetMoonPlanetarium) 0.0)
  (EventDispatchers|AssignOnAudioFinished (Variables|Default|GetMoonPlanetarium) (delegate Custom|StartMoving)))

(event Custom|PlayJupiterAudio
  (bind _jupiterplanetarium (Variables|Default|GetJupiterPlanetarium))
  (Audio|Components|Audio|Play _jupiterplanetarium 0.0)
  (EventDispatchers|AssignOnAudioFinished _jupiterplanetarium (delegate Custom|StartMoving2)))

(event Custom|StopMoving
  (Variables|Default|SetCurrentRotation (Variables|/Script/Engine.SceneComponent|GetRelativeRotation (Variables|Default|GetRotunda)))
  (Utilities|FlowControl|Sequence
    (:then_0
      (bind _rotationrate (Timeline|Timeline Stop)
        (:Update
          (Transformation|SetRelativeRotation (Variables|Default|GetRotunda) (Math|Rotator|Lerp(Rotator) (Variables|Default|GetStartRotation) (Variables|Default|GetEndRotation) _rotationrate) false false))))
    (:then_1
      (bind _slowrate (Timeline|StopTimeline Play)
        (:Update
          (Transformation|SetRelativeRotation (Variables|Default|GetRotunda) (Math|Rotator|Lerp(Rotator) (Variables|Default|GetCurrentRotation) (Variables|Default|GetMoonRotation) _slowrate) false false)
          (Widget|RemovefromParent (Variables|Default|GetSpaceWidgetRef)))
        (:Finished
          (Variables|Default|SetMoonFinished true)
          (Utilities|FlowControl|Delay 0.3)
          (bind _returnvalue (Actor|GetActorOfClass "/Game/FirstPerson/Blueprints/BP_FirstPersonCharacter.BP_FirstPersonCharacter_C"))
          (Default|JupiterMiniGame _returnvalue))))))

(event Custom|StartMoving2
  (Rendering|SetVisibility (Variables|Default|GetJupiter) true false)
  (bind _returnvalue (UserInterface|CreateWidget "/Game/Widgets/SpacebarIcon.SpacebarIcon_C"))
  (Variables|Default|SetSpaceWidgetRef _returnvalue)
  (UserInterface|Viewport|AddtoViewport _returnvalue 0)
  (bind _rotationrate (Timeline|Timeline_0 Play)
    (:Update
      (Transformation|SetRelativeRotation (Variables|Default|GetRotunda) (Math|Rotator|Lerp(Rotator) (Variables|Default|GetMoonRotation) (Math|Rotator|MakeRotator 0.0 0.0 (+ (.yaw (Variables|Default|GetMoonRotation)) 3.6e+02)) _rotationrate) false false))))

(event Custom|ResetCamera
  (Default|ResetCamera (Variables|Default|GetFirstPersonCharRef)))

(event EventTick
  (params (DeltaSeconds :type Float%20%28single-precision%29)))

(event EventBeginPlay
  (bind _returnvalue (Actor|GetActorOfClass "/Game/FirstPerson/Blueprints/CameraPeatBP.CameraPeatBP_C"))
  (Variables|Default|SetCameraPeatRef _returnvalue)
  (bind _returnvalue_2 (Actor|GetActorOfClass "/Game/FirstPerson/Blueprints/BP_FirstPersonCharacter.BP_FirstPersonCharacter_C"))
  (Variables|Default|SetFirstPersonCharRef _returnvalue_2)
  (bind _returnvalue_3 (Actor|GetActorOfClass "/Game/FirstPerson/Blueprints/TextRenderJupiterBP.TextRenderJupiterBP_C"))
  (Variables|Default|SetJupiterTextRef _returnvalue_3)
  (bind _returnvalue_4 (Actor|GetActorOfClass "/Game/FirstPerson/Blueprints/TextRenderMoonBP.TextRenderMoonBP_C"))
  (Variables|Default|SetMoonTextRef _returnvalue_4)
  (bind _returnvalue_5 (Actor|GetActorOfClass "/Game/FirstPerson/Blueprints/LandscapeLift.LandscapeLift_C"))
  (Variables|Default|SetLandscapeLiftRef _returnvalue_5)
  (bind _returnvalue_6 (Actor|GetActorOfClass "/Game/FirstPerson/Blueprints/Timer.Timer_C"))
  (Variables|Default|SetTimerRef _returnvalue_6))

(fn ConstructionScript)